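; Player pawn with axis-driven movement and look that emits noise from both its footsteps and the player's real microphone input.
; Raw WASD key events feed ApplyStepSound, which toggles the footstep sound and IsWalking.
; AudioCapture's envelope callback sets an amplified, capped mic volume.
; Every Tick adds a fixed walking volume to it and reports the total through PawnNoiseEmitter at the pawn's location, capped while walking.
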(event `self.ReceiveBeginPlay`
  (`AudioComponent.Stop` (`self.FootStepSound`))
  (set `self.MicVolume` 0.0))

(event `InputAxis|Turn`
  (params (AxisValue :type "Float (single-precision)"))
  (`self.AddControllerYawInput` AxisValue))

(event `Key|S`
  (params (Key :type "Key Structure"))
  (:`Pressed`
    (set `self.S Pressed` true)
    (`self.ApplyStepSound`))
  (:`Released`
    (set `self.S Pressed` false)
    (`self.ApplyStepSound`)))

(event `Key|W`
  (params (Key :type "Key Structure"))
  (:`Pressed`
    (set `self.W Pressed` true)
    (`self.ApplyStepSound`))
  (:`Released`
    (set `self.W Pressed` false)
    (`self.ApplyStepSound`)))

(event `InputAxis|LookUp`
  (params (AxisValue :type "Float (single-precision)"))
  (`self.AddControllerPitchInput` AxisValue))

(event `Key|D`
  (params (Key :type "Key Structure"))
  (:`Pressed`
    (set `self.D Pressed` true)
    (`self.ApplyStepSound`))
  (:`Released`
    (set `self.D Pressed` false)
    (`self.ApplyStepSound`)))

(event `Key|A`
  (params (Key :type "Key Structure"))
  (:`Pressed`
    (set `self.A Pressed` true)
    (`self.ApplyStepSound`))
  (:`Released`
    (set `self.A Pressed` false)
    (`self.ApplyStepSound`)))

(event `self.ReceiveTick`
  (params (DeltaSeconds :type "Float (single-precision)"))
  (bind _returnvalue (+ (`self.MicVolume`) (`self.StepVolume`)))
  (if (`self.IsWalking`)
    (set `self.StepVolume` 0.3)
    (if (> _returnvalue 1.0)
      (set `self.TotalNoiseVolume` 1.0)
      (else
        (set `self.TotalNoiseVolume` _returnvalue :!label _label)))
    (else
      (set `self.StepVolume` 0.0)
      (goto _label)))
  (`PawnNoiseEmitterComponent.MakeNoise` (`self.PawnNoiseEmitter`) self (`self.TotalNoiseVolume`) (`self.K2_GetActorLocation`)))

(event `InputAxis|MoveForward`
  (params (AxisValue :type "Float (single-precision)"))
  (bind _output_get (set `self.Move Forward` AxisValue))
  (`self.AddMovementInput` (`self.GetActorForwardVector`) _output_get))

(event `self.AudioCapture.OnAudioEnvelopeValue`
  (params (EnvelopeValue :type "Float (single-precision)"))
  (bind _returnvalue (* EnvelopeValue 5.0))
  (if (> _returnvalue 1.0)
    (set `self.MicVolume` 1.0)
    (else
      (set `self.MicVolume` _returnvalue))))

(event `InputAxis|MoveRight`
  (params (AxisValue :type "Float (single-precision)"))
  (bind _output_get (set `self.Move Right` AxisValue))
  (`self.AddMovementInput` (`self.GetActorRightVector`) _output_get))

(fn `ApplyStepSound`
  (if (or (`self.W Pressed`) (`self.A Pressed`) (`self.S Pressed`) (`self.D Pressed`))
    (`AudioComponent.Play` (`self.FootStepSound`) 0.5)
    (set `self.IsWalking` true)
    (else
      (`AudioComponent.Stop` (`self.FootStepSound`))
      (set `self.IsWalking` false))))

(fn `UserConstructionScript`)