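; Player character pawn that handles first-person-style movement, mouse look and looping footstep audio.
; Axis inputs drive forward and right movement along the actor's vectors and feed controller yaw and pitch.
; W, A, S and D key events track held flags and call ApplyStepSound, which plays the footstep sound while any is held and stops it otherwise.
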(event `self.ReceiveBeginPlay`
  (`AudioComponent.Stop` (`self.FootStepSound`)))

(event `InputAxis|Turn`
  (params (AxisValue :type "Float (single-precision)"))
  (`self.AddControllerYawInput` AxisValue))

(event `Key|S`
  (params (Key :type "Key Structure"))
  (:`Pressed`
    (set `self.S Pressed` true)
    (`self.ApplyStepSound`))
  (:`Released`
    (set `self.S Pressed` false)
    (`self.ApplyStepSound`)))

(event `Key|W`
  (params (Key :type "Key Structure"))
  (:`Pressed`
    (set `self.W Pressed` true)
    (`self.ApplyStepSound`))
  (:`Released`
    (set `self.W Pressed` false)
    (`self.ApplyStepSound`)))

(event `InputAxis|LookUp`
  (params (AxisValue :type "Float (single-precision)"))
  (`self.AddControllerPitchInput` AxisValue))

(event `Key|D`
  (params (Key :type "Key Structure"))
  (:`Pressed`
    (set `self.D Pressed` true)
    (`self.ApplyStepSound`))
  (:`Released`
    (set `self.D Pressed` false)
    (`self.ApplyStepSound`)))

(event `Key|A`
  (params (Key :type "Key Structure"))
  (:`Pressed`
    (set `self.A Pressed` true)
    (`self.ApplyStepSound`))
  (:`Released`
    (set `self.A Pressed` false)
    (`self.ApplyStepSound`)))

(event `self.ReceiveTick`
  (params (DeltaSeconds :type "Float (single-precision)")))

(event `InputAxis|MoveForward`
  (params (AxisValue :type "Float (single-precision)"))
  (bind _output_get (set `self.Move Forward` AxisValue))
  (`self.AddMovementInput` (`self.GetActorForwardVector`) _output_get))

(event `InputAxis|MoveRight`
  (params (AxisValue :type "Float (single-precision)"))
  (bind _output_get (set `self.Move Right` AxisValue))
  (`self.AddMovementInput` (`self.GetActorRightVector`) _output_get))

(fn `ApplyStepSound`
  (if (or (`self.W Pressed`) (`self.A Pressed`) (`self.S Pressed`) (`self.D Pressed`))
    (`AudioComponent.Play` (`self.FootStepSound`) 0.5)
    (else
      (`AudioComponent.Stop` (`self.FootStepSound`)))))

(fn `UserConstructionScript`)