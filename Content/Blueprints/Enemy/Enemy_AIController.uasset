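; Enemy AI controller that sets up the enemy's blackboard and runs its behavior tree.
; On BeginPlay it seeds Enemy_AI_BB with the pawn's home location, an idle time and a random navigable target near the start point, then starts Enemy_AI_BT.
; PawnSensing hearing writes the noise volume and location to the blackboard as the noticed player position, resetting the volume to zero after a short delay.
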(event `self.ReceiveBeginPlay`
  (bind _returnvalue (`self.K2_GetActorLocation` (`self.K2_GetPawn`)))
  (`|ExecutionSequence`
    (:`then_0`
      (`self.UseBlackboard` "/Game/Blueprints/Enemy/Enemy_AI_BB.Enemy_AI_BB")
      (`BlackboardComponent.SetValueAsVector` (`self.Blackboard`) (`self.HomeLoc Key`) _returnvalue)
      (`BlackboardComponent.SetValueAsFloat` (`self.Blackboard`) (`self.Idle Time Key`) 1.0)
      (`BlackboardComponent.SetValueAsVector` (`self.Blackboard`) (`self.Target Loc Key`) (`NavigationSystemV1.K2_GetRandomLocationInNavigableRadius` _returnvalue 1000.0 null null))
      (`BlackboardComponent.SetValueAsFloat` (`self.Blackboard`) (`self.PlayerNoiseVolume Key`) 0.0))
    (:`then_1`
      (`self.RunBehaviorTree` "/Game/Blueprints/Enemy/Enemy_AI_BT.Enemy_AI_BT"))))

(event `self.PawnSensing.OnHearNoise`
  (params (Instigator :type "Pawn Object Reference") (Location :type "Vector Structure (by ref)") (Volume :type "Float (single-precision)"))
  (`self.UseBlackboard` "/Game/Blueprints/Enemy/Enemy_AI_BB.Enemy_AI_BB")
  (`BlackboardComponent.SetValueAsFloat` (`self.Blackboard`) (`self.PlayerNoiseVolume Key`) Volume)
  (`BlackboardComponent.SetValueAsVector` (`self.Blackboard`) (`self.NoticedPlayerLocation Key`) Location)
  (`KismetSystemLibrary.Delay` 1.0)
  (`BlackboardComponent.SetValueAsFloat` (`self.Blackboard`) (`self.PlayerNoiseVolume Key`) 0.0))

(fn `UserConstructionScript`)